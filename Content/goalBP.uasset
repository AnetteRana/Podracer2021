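; Goal marker Blueprint that acts as either an "A" start point or a "B" end point for a game run.
; On BeginPlay, the IsA flag sets both text renders to show "A" or "B".
; When a PawnBP overlaps the static mesh, it calls that pawn's start-game dispatcher for A or its end-game dispatcher for B.
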(event OnComponentBeginOverlap(StaticMesh)
  (params (OverlappedComponent :type Primitive%20Component%20Object%20Reference) (OtherActor :type Actor%20Object%20Reference) (OtherComp :type Primitive%20Component%20Object%20Reference) (OtherBodyIndex :type Integer) (bFromSweep :type Boolean) (SweepResult :type Hit%20Result%20Structure%20%28by%20ref%29))
  (bind _aspawn_bp (Utilities|Casting|CastToPawnBP OtherActor))
  (if (Utilities|IsValid _aspawn_bp)
    (if (Variables|Default|GetisA)
      (Default|CallStartGameDispatcher _aspawn_bp)
      (else
        (Default|CallEndGameDispatcher _aspawn_bp)))))

(event EventBeginPlay
  (bind _returnvalue (Utilities|Text|MakeLiteralText "B"))
  (bind _returnvalue_2 (Utilities|Text|MakeLiteralText "A"))
  (bind _textrender (Variables|Default|GetTextRender))
  (bind _textrender1 (Variables|Default|GetTextRender1))
  ;[1 1 1] set text A/B
  (if (Variables|Default|GetisA)
    (Rendering|Components|TextRender|SetText _textrender1 _returnvalue_2)
    (Rendering|Components|TextRender|SetText _textrender _returnvalue_2)
    (else
      (Rendering|Components|TextRender|SetText _textrender1 _returnvalue)
      (Rendering|Components|TextRender|SetText _textrender _returnvalue))))

(fn ConstructionScript)