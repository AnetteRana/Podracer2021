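; A pawn that drives along its forward vector and yaws from move inputs, using a FloatingPawnMovement component.
; Each Tick it traces 1000 units down, pushing upward on a hit and otherwise easing its roll back to level.
; UpdateBody is called every frame but is empty; the body offset by velocity and the overlap-based ground check are left disconnected.
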(event Custom|updateBody)

(event EventTick
  (params (DeltaSeconds :type Float%20%28single-precision%29))
  (bind _returnvalue (Transformation|GetActorLocation))
  (bind _returnvalue_2 (Transformation|GetActorRotation))
  (bind (_roll _pitch _yaw) (Math|Rotator|BreakRotator _returnvalue_2))
  (Class|PawnMovementComponent|AddInputVector (Variables|Default|GetFloatingPawnMovement) (* (Transformation|GetActorForwardVector) (Input|AxisValues|GetMoveForward)) false)
  (Class|Actor|AddActorWorldRotation self (Math|Rotator|MakeRotator 0.0 0.0 (* (Input|AxisValues|GetMoveRight) 1.0)))
  (CallFunction|UpdateBody)
  ;[1 1 1] is ground near? (under)
  (bind _returnvalue_3 (Collision|LineTraceByChannel _returnvalue (- _returnvalue "0, 0,1000.000000") "TraceTypeQuery1" false 0 "None"))
  (if _returnvalue_3
    ;[1 1 1] higher
    (Class|PawnMovementComponent|AddInputVector (Variables|Default|GetFloatingPawnMovement) (Math|Vector|MakeVector 0.0 0.0 1.0) false)
    (else
      (Transformation|SetActorRotation (Math|Rotator|Lerp(Rotator) _returnvalue_2 (Math|Rotator|MakeRotator 0.0 _pitch _yaw) 0.5 true)))))

(fn ConstructionScript)